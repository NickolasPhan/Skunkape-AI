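; Sasquatch AI NPC that takes voice or typed prompts and replies with ElevenLabs speech through the AIITK component.
; Recorded audio goes to Whisper, and the transcript goes to GPT, or straight to ElevenLabs in parrot mode, with messages appended to the chat params.
; Standard or streamed audio plays on VoiceBox, driving a talking flag, random emote and subtitles.
; A combo box filled from fetched ElevenLabs voices sets the speaking voice.
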(event 3DButtonReleased(CaptureVoiceButton)
  (bind _aiitkcomponentbp (Variables|Default|GetAIITKComponentBP))
  (bind _capturevoicebutton (Variables|Default|GetCaptureVoiceButton))
  ;[0 0 0] Buttons
  (Utilities|FlowControl|FlipFlop
    (:A
      (Default|StartAudioCapture _aiitkcomponentbp)
      (Variables|Data|SetVoiceFilePath "")
      (Rendering|Material|SetMaterial _capturevoicebutton 1 "/AIIntegrationToolkit/Examples/Assets/Materials/Instances/HighlightPulseRed.HighlightPulseRed"))
    (:B
      (Default|StopAudioCaptureandSave _aiitkcomponentbp "TempVoice")
      (Rendering|Material|SetMaterial _capturevoicebutton 1 "/AIIntegrationToolkit/Examples/Assets/Materials/Instances/ChatBoyPrimary.ChatBoyPrimary"))))

(event OnAudioCaptureSaved(AIITKComponentBP)
  (params (WAVFilePath :type String))
  ;[0 0 0] Whisper request
  (bind _output_get (Variables|Data|SetVoiceFilePath WAVFilePath))
  (bind _structout (Utilities|Struct|SetmembersinWhisperAPIParams (Variables|Options|GetWhisperParams) _output_get))
  (Default|SendRequesttoWhisper (Variables|Default|GetAIITKComponentBP) _structout)
  (Utilities|Struct|Setmembersin11LabsRequiredParams (Utilities|Struct|Break11LabsRequestParams (Variables|Options|Get11LabsParams)) (Variables|Data|GetVoiceFilePath)) ; For Speech To Speech
)

(event OnAudioGenerated(AIITKComponentBP)
  (params (GeneratedAudio :type Sound%20Wave%20Object%20Reference) (RawAudioData :type Array%20of%20Bytes))
  (bind _voicebox (Variables|Default|GetVoiceBox))
  ;[0 0 0] Speak Streamed/Standard
  (Utilities|CheckifStreamed
    (:Standard
      (Audio|Components|Audio|SetSound _voicebox GeneratedAudio)
      (Audio|Components|Audio|Play _voicebox 0.0)
      (CallFunction|StartTalking))))

(event OnError(AIITKComponentBP)
  (params (ErrorMessage :type String))
  ;[0 0 0] Speak Streamed/Standard
  (Development|PrintString ErrorMessage true true "(R=1.000000,G=0.000000,B=0.036017,A=1.000000)" 1e+01))

(event OnWhisperTranscriptGenerated(AIITKComponentBP)
  (params (Transcription :type String))
  ;[0 0 0] Whisper response
  (bind _output_get (Variables|Data|SetCurrentTranscription Transcription))
  (Utilities|SetPromptText _output_get)
  (if (Variables|Data|GetParrotMode)
    (bind _structout (Utilities|Struct|Setmembersin11LabsRequestParams (Variables|Options|Get11LabsParams) (Variables|Data|GetCurrentTranscription)))
    (Default|SendRequestto11Labs (Variables|Default|GetAIITKComponentBP) _structout)
    (Variables|Data|SetCurrentResponse (Variables|Data|GetCurrentTranscription))
    (Audio|PlaySound2D "/AIIntegrationToolkit/Examples/Assets/Audio/SoundWaves/Send8Bit.Send8Bit" 1.0 1.0 0.0 0 0)
    (else
      (CallFunction|AddGPTMessage (Variables|Options|GetGPTParams) (Variables|Data|GetCurrentTranscription))
      (Default|SendRequesttoGPT (Variables|Default|GetAIITKComponentBP) (Variables|Options|GetGPTParams)))))

(event OnAudioInitialized(AIITKComponentBP)
  (params (NewSoundWave :type Sound%20Wave%20Procedural%20Object%20Reference))
  (bind _voicebox (Variables|Default|GetVoiceBox))
  ;[0 0 0] Speak Streamed/Standard
  (Utilities|CheckifStreamed
    (:Streamed
      (Audio|Components|Audio|SetSound _voicebox NewSoundWave)
      (Audio|Components|Audio|Play _voicebox 0.0))))

(event OnGPTCompleted(AIITKComponentBP)
  (params (Completion :type GPT%20Chat%20Completion%20Structure))
  ;[0 0 0] GPT response
  (bind _output_get (Variables|Data|SetCurrentResponse (Class|OpenAIFunctionLibrary|GetMessageContent (Class|OpenAIFunctionLibrary|GetResponseMessage Completion))))
  (bind _structout (Utilities|Struct|Setmembersin11LabsRequestParams (Variables|Options|Get11LabsParams) _output_get))
  (Default|SendRequestto11Labs (Variables|Default|GetAIITKComponentBP) _structout)
  (Audio|PlaySound2D "/AIIntegrationToolkit/Examples/Assets/Audio/SoundWaves/Send8Bit.Send8Bit" 1.0 1.0 0.0 0 0)
  (if (not (Variables|Data|GetParrotMode))
    (CallFunction|AddGPTMessage (Variables|Options|GetGPTParams) (Variables|Data|GetCurrentResponse))))

(event 3DButtonReleased(TextButton)
  (bind _sasquatchpromptbubbleref (Variables|Data|GetSasquatchPromptBubbleRef))
  (bind _elevenpromptbox (Variables|/Game/Sasquatch_AI_Map/Blueprints/Widgets/Sasquatch_PromptBubble_WBP.Sasquatch_PromptBubble_WBP_C|GetElevenPromptBox _sasquatchpromptbubbleref))
  ;[0 0 0] Buttons
  (if (Widget|IsVisible _sasquatchpromptbubbleref)
    (Widget|RemovefromParent _sasquatchpromptbubbleref)
    (Rendering|Components|TextRender|SetText _elevenpromptbox "")
    (else
      (UserInterface|Viewport|AddtoViewport _sasquatchpromptbubbleref 0)
      (Widget|SetKeyboardFocus _elevenpromptbox))))

(event OnProcAudioGenerated(AIITKComponentBP)
  (params (GeneratedAudio :type Sound%20Wave%20Procedural%20Object%20Reference) (RawAudioData :type Array%20of%20Bytes))
  ;[0 0 0] Speak Streamed/Standard
  (Utilities|CheckifStreamed
    (:Streamed
      (Utilities|FlowControl|DoOnce false
        (:Completed
          (CallFunction|StartTalking))))))

(event OnAudioFinished(AIITKComponentBP)
  ;[0 0 0] Speak Streamed/Standard
  (CallFunction|StopTalking)
  (Utilities|FlowControl|DoOnce false) ; enters at Reset
)

(event Custom|StartTalking
  ;[0 0 0] Speak Streamed/Standard
  (Utilities|StartTalkFX))

(event Custom|TextPromptSubmit
  ;[0 0 0] Whisper response
  (if (Variables|Data|GetParrotMode)
    (bind _structout (Utilities|Struct|Setmembersin11LabsRequestParams (Variables|Options|Get11LabsParams) (Variables|Data|GetCurrentTranscription)))
    (Default|SendRequestto11Labs (Variables|Default|GetAIITKComponentBP) _structout)
    (Variables|Data|SetCurrentResponse (Variables|Data|GetCurrentTranscription))
    (Audio|PlaySound2D "/AIIntegrationToolkit/Examples/Assets/Audio/SoundWaves/Send8Bit.Send8Bit" 1.0 1.0 0.0 0 0)
    (else
      (CallFunction|AddGPTMessage (Variables|Options|GetGPTParams) (Variables|Data|GetCurrentTranscription))
      (Default|SendRequesttoGPT (Variables|Default|GetAIITKComponentBP) (Variables|Options|GetGPTParams)))))

(event Custom|StopTalking
  ;[0 0 0] Speak Streamed/Standard
  (Utilities|StopTalkFX))

(event EventBeginPlay
  (|Init))

(fn ConstructionScript)

(fn SelectRandomEmote
  (Variables|Data|SetCurrentEmote (.OutItem (Utilities|Array|Random (Variables|Data|GetEmoteList))))
  (return))

(fn AddGPTMessage
  (params (GPTChatPromptParams :type GPT%20Chat%20Prompt%20Params%20Structure%20%28by%20ref%29) (Content :type String))
  (Utilities|Array|Add (Utilities|Struct|BreakGPTChatPromptParams GPTChatPromptParams) (Utilities|Struct|MakeGPTChatMessage "user" (Utilities|Struct|MakeUserMessage (Utilities|Array|MakeArray (Utilities|Struct|MakeContentPart Content))))))

(event On11LabsVoicesStored(AIITKComponentBP)
  (params (StoredVoices :type Map%20of%20Strings%20to%20Strings))
  (bind _assasquatch_voice_combo_box_wbp (Utilities|Casting|CastToSasquatch_VoiceComboBox_WBP (UserInterface|GetWidget (Variables|Default|GetVoiceChoice))))
  (Default|PopulateComboBox _assasquatch_voice_combo_box_wbp StoredVoices)
  (EventDispatchers|BindEventtoOnSelectionChanged (Variables|/Game/Sasquatch_AI_Map/Blueprints/Widgets/Sasquatch_VoiceComboBox_WBP.Sasquatch_VoiceComboBox_WBP_C|GetVoiceChoices _assasquatch_voice_combo_box_wbp) (delegate Custom|UpdateSelection))
  (Class|ComboBoxString|SetSelectedIndex (Variables|/Game/Sasquatch_AI_Map/Blueprints/Widgets/Sasquatch_VoiceComboBox_WBP.Sasquatch_VoiceComboBox_WBP_C|GetVoiceChoices _assasquatch_voice_combo_box_wbp)))

(event On11LabsModelsStored(AIITKComponentBP)
  (params (StoredModels :type Map%20of%20Strings%20to%20Strings))
  (Development|PrintString (Class|OpenAIFunctionLibrary|PrintStringMap StoredModels) true true "(R=0.000000,G=1.000000,B=0.067130,A=1.000000)"))

(event Custom|UpdateSelection
  (params (SelectedItem :type String) (SelectionType :type ESelectInfo%20Enum :default "OnKeyPress"))
  (Utilities|Struct|Setmembersin11LabsRequiredParams (Utilities|Struct|Break11LabsRequestParams (Variables|Options|Get11LabsParams)) (.Value (Utilities|Map|Find (Variables|/AIIntegrationToolkit/Core/AIITKComponentBP.AIITKComponentBP_C|GetCurrent11LabsVoices (Variables|Default|GetAIITKComponentBP)) SelectedItem))))

(event Custom|EnterPressed
  (params (Prompt :type String))
  (Variables|Data|SetCurrentTranscription Prompt)
  (CallFunction|TextPromptSubmit)
  (Rendering|Components|TextRender|SetText (Variables|/Game/Sasquatch_AI_Map/Blueprints/Widgets/Sasquatch_PromptBubble_WBP.Sasquatch_PromptBubble_WBP_C|GetElevenPromptBox (Variables|Data|GetSasquatchPromptBubbleRef)) ""))